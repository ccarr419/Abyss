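; The mouseLight Blueprint moves a spotlight to follow the player's mouse cursor in the world.
; Each Tick deprojects the cursor position and projects it along the view ray by LightScrollValue.
; The spotlight takes X and Z from that point, while Y is pinned to LightDistance, keeping the light on a fixed plane.
; Both values are set on BeginPlay and stay constant in this graph, with no scroll input handled.
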(event EventBeginPlay
  (Variables|Default|SetlightScrollValue 825.0)
  (Variables|Default|SetlightDistance 1.5e+02))

(event EventTick
  (params (DeltaSeconds :type Float%20%28single-precision%29))
  (bind _returnvalue (Game|GetPlayerController 0))
  (bind _lightscrollvalue (Variables|Default|GetlightScrollValue))
  (bind (_worldlocation _worlddirection) (Game|Player|ConvertMouseLocationToWorldSpace _returnvalue))
  (bind _returnvalue_2 (* _worlddirection _lightscrollvalue))
  (bind _returnvalue_3 (+ _worldlocation _returnvalue_2))
  (bind (_x _y _z) (Math|Vector|BreakVector _returnvalue_3))
  (Transformation|SetWorldLocation (Variables|Default|GetSpotLight) (Math|Vector|MakeVector _x (Variables|Default|GetlightDistance) _z) false false))

(fn ConstructionScript)