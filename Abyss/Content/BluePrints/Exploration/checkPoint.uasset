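; Exploration checkpoint that lights as a sword-in-fire bonfire when the player first overlaps it.
; Activation swaps the flipbook, sets light and particle templates, plays an ignite sound, and records itself as LastCheckpoint in AbyssGameInstance.
; Tick keeps the crackle audio in step with the checkpoint state.
; Tick also flickers the light's intensity and blue channel through a randomly delayed FlipFlop, regardless of activation.
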(event EventBeginPlay
  ;[1 1 1] Main
  (Variables|Default|SetcheckpointSet false)
  (Variables|Default|SetfireBrightness 256.0)
  (Variables|Default|SetfireRadius 512.0)
  (Variables|Default|SetmaxBrightness 512.0)
  (Variables|Default|SetmaxVolume 2.0)
  (bind _output_get (Variables|Default|SetcurrentVolume 1.0))
  (Audio|Components|Audio|SetVolumeMultiplier (Variables|Default|GetFire%20Crackle) _output_get :!class /Script/Engine.AudioComponent))

(event Collision|EventActorBeginOverlap
  (params (OtherActor :type Actor%20Object%20Reference))
  (bind _fire_light (Variables|Default|GetFire%20Light))
  ;[1 1 1] Set Checkpoint
  (if (== OtherActor (Game|GetPlayerCharacter 0))
    (if (not (Variables|Default|GetcheckpointSet))
      (Variables|Default|SetcheckpointSet true)
      (Sprite|SetFlipbook (Variables|Default|GetCheckpointFlipbook) "/Game/Assets/Sprites/Other/swordFire.swordFire")
      (Rendering|Components|Light|SetIntensity _fire_light (Variables|Default|GetfireBrightness))
      (Rendering|Lighting|SetAttenuationRadius _fire_light (Variables|Default|GetfireRadius))
      (bind _asabyss_game_instance (Utilities|Casting|CastToAbyssGameInstance (Game|GetGameInstance)))
      (Variables|Default|SetgameInstanceAtCheckpoint _asabyss_game_instance)
      (Variables|/Game/BluePrints/AbyssGameInstance.AbyssGameInstance_C|SetlastCheckpoint _asabyss_game_instance self)
      (Audio|PlaySound2D "/Game/Assets/Sounds/fireIgnite.fireIgnite" (Variables|Default|GetcurrentVolume))
      (Effects|Components|ParticleSystem|SetTemplate (Variables|Default|GetFire%20Embers) "/Game/Assets/Paricles/fireSpark.fireSpark")
      (Effects|Components|ParticleSystem|SetTemplate (Variables|Default|GetFire%20Smoke) "/Game/Assets/Paricles/fireSmoke.fireSmoke")
      (Development|PrintString "Checkpoint!" true true "(R=1.000000,G=0.000000,B=0.000000,A=1.000000)" 4.0))))

(event EventTick
  (params (DeltaSeconds :type Float%20%28single-precision%29))
  (bind _fire_light (Variables|Default|GetFire%20Light))
  (bind _fire_crackle (Variables|Default|GetFire%20Crackle))
  (bind _returnvalue (Audio|Components|Audio|IsPlaying _fire_crackle))
  (bind _returnvalue_2 (Rendering|Components|Light|GetLightColor _fire_light))
  (bind _intensity (Variables|/Script/Engine.LightComponentBase|GetIntensity _fire_light))
  (bind (_r _g _b _a) (Utilities|Struct|BreakLinearColor _returnvalue_2))
  ;[1 1 1] Fire Light Flicker and Sound Effects
  (Utilities|FlowControl|Sequence
    (:then_0
      (if (Variables|Default|GetcheckpointSet)
        (if (not _returnvalue)
          (Audio|Components|Audio|Play _fire_crackle 0.0))
        (elif _returnvalue
          (Audio|Components|Audio|Stop _fire_crackle))))
    (:then_1
      (Utilities|FlowControl|Delay (Math|Random|RandomFloatinRange 0.1 0.6))
      (Utilities|FlowControl|FlipFlop
        (:A
          (Rendering|Components|Light|SetIntensity _fire_light (* _intensity 1.15))
          (Rendering|Components|Light|SetLightColor _fire_light (Math|Color|MakeColor _r _g (- _b 0.05) _a) true))
        (:B
          (Rendering|Components|Light|SetIntensity _fire_light (/ _intensity 1.15))
          (Rendering|Components|Light|SetLightColor _fire_light (Math|Color|MakeColor _r _g (+ _b 0.05) _a) true))))))

(fn ConstructionScript)