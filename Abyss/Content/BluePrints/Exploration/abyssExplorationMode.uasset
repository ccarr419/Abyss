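; Game mode for Abyss exploration that sets up the mouse cursor, lighting and ambient music when play begins.
; BeginPlay spawns a MouseLight actor at a fixed transform, shows the cursor and starts the ambient background track as a 2D sound.
; It then sets the volume levels and copies them, with the track and its audio reference, into AbyssGameInstance through changeInstanceValues.
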(event Custom|changeInstanceValues
  ;[1 1 1] SetInstanceValues
  (bind _asabyss_game_instance (Utilities|Casting|CastToAbyssGameInstance (Game|GetGameInstance)))
  (Variables|/Game/BluePrints/AbyssGameInstance.AbyssGameInstance_C|SetmaxVolume _asabyss_game_instance (Variables|Default|GetmaxVolume))
  (Variables|/Game/BluePrints/AbyssGameInstance.AbyssGameInstance_C|SetmusicVolume _asabyss_game_instance (Variables|Default|GetmusicVolume))
  (Variables|/Game/BluePrints/AbyssGameInstance.AbyssGameInstance_C|SetbackgroundMusic _asabyss_game_instance (Variables|Default|GetbackgroundMusic))
  (Variables|/Game/BluePrints/AbyssGameInstance.AbyssGameInstance_C|SetmusicReference _asabyss_game_instance (Variables|Default|GetmusicReference)))

(event EventBeginPlay
  ;[1 1 1] Main
  (Game|SpawnActorfromClass "/Game/BluePrints/Exploration/mouseLight.mouseLight_C" (Math|Transform|MakeTransform "0.000000,630.000000, 0" "0.000000,-100.000000, 0") "Undefined" 0 0)
  (Variables|/Script/Engine.PlayerController|SetbShowMouseCursor (Game|GetPlayerController 0) true)
  (bind _output_get (Variables|Default|SetbackgroundMusic "/Game/Assets/Sounds/ambientBackground.ambientBackground"))
  (bind _returnvalue (Audio|SpawnSound2D _output_get 1.0 1.0 0.0 0 true))
  (Variables|Default|SetmusicReference _returnvalue)
  (Variables|Default|SetmusicVolume 0.7)
  (Variables|Default|SetmaxVolume 2.8)
  (CallFunction|ChangeInstanceValues))

(fn ConstructionScript)