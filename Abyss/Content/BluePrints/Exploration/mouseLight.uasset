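; Exploration light that follows the mouse cursor, with a flickering spotlight.
; BeginPlay sets the light's intensity, radius and placement values.
; Tick moves the spotlight to GetMouseLocation, whose graph deprojects the cursor along its world direction and substitutes a fixed Y depth.
; Tick also drives the flicker, where a random Delay feeds a FlipFlop that alternately raises and restores intensity and blue tint.
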(event EventBeginPlay
  ;[1 1 1] Main Startup
  (Utilities|SetInitialVariables))

(event EventTick
  (params (DeltaSeconds :type Float%20%28single-precision%29))
  ;[1 1 1] Tick - Light Position
  (Transformation|SetWorldLocation (Variables|Default|GetSpotLight) (Utilities|GetMouseLocation) false false)
  (Utilities|FlickerMouseLight))

(fn ConstructionScript)