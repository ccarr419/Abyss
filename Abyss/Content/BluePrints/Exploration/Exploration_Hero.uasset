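; Exploration_Hero is the side-view flipbook knight the player controls during exploration, with stats, HUD, pause menu and debug stat keys.
; Tick restores position, disabled battle triggers, torches and checkpoint fire from AbyssGameInstance after battles, and drives animation, facing, looping movement sounds and spotlight flicker.
; Axis inputs feed movement and an onLadder event, which re-checks every 0.1 seconds, switching between Flying and Walking for climbing.
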(event Custom|onLadder
  (bind _charactermovement (Variables|Character|GetCharacterMovement))
  ;[1 1 1] Climbing
  (bind _isonladder (Utilities|IsOverlappingLadder :!label _label)
    (:Exit
      (if _isonladder
        (if (!= (Variables|Default|GetclimbScaleValue) 0.0)
          (Pawn|Components|CharacterMovement|SetMovementMode _charactermovement "MOVE_Flying" 0)
          (Variables|/Script/Engine.MovementComponent|SetVelocity _charactermovement (* (Math|Vector|MakeVector (Variables|Default|GetmoveScaleValue) 0.0 (Variables|Default|GetclimbScaleValue)) (Variables|Default|GetclimbVelocityVector)))
          (Variables|Default|SetisOnLadder true)
          (Utilities|FlowControl|Delay 0.1)
          (goto _label)
          (else
            _)))
      (Pawn|Components|CharacterMovement|SetMovementMode _charactermovement "MOVE_Walking" 0)
      (Variables|Default|SetisOnLadder false))))

(event Custom|checkReturnFromBattle
  ;[1 1 1] Reset Player Location
  (bind _asabyss_game_instance (Utilities|Casting|CastToAbyssGameInstance (Game|GetGameInstance)))
  (if (Variables|/Game/BluePrints/AbyssGameInstance.AbyssGameInstance_C|GetinBattle _asabyss_game_instance)
    (Variables|/Game/BluePrints/AbyssGameInstance.AbyssGameInstance_C|SetinBattle _asabyss_game_instance false)
    (for _array_element (Variables|/Game/BluePrints/AbyssGameInstance.AbyssGameInstance_C|GetbattleTriggerIds _asabyss_game_instance)
      (bind _outactors (Actor|GetAllActorsOfClass "/Game/BluePrints/Exploration/Fort_BattleTrigger.Fort_BattleTrigger_C"))
      (Variables|/Script/Engine.PrimitiveComponent|SetbGenerateOverlapEvents (Variables|/Script/Engine.TriggerBase|GetCollisionComponent (Utilities|Array|Get(acopy) _outactors _array_element)) false))
    (Transformation|SetWorldTransform (Variables|/Script/Engine.Character|GetCapsuleComponent (Game|GetPlayerCharacter 0)) (Variables|/Game/BluePrints/AbyssGameInstance.AbyssGameInstance_C|GetlastPlayerBattlePositon _asabyss_game_instance) false false)
    (CallFunction|RelightTorches)
    (CallFunction|RelightLastCheckpoint)))

(event Custom|relightLastCheckpoint
  ;[1 1 1] Relight Last Checkpoint
  (bind _asabyss_game_instance (Utilities|Casting|CastToAbyssGameInstance (Game|GetGameInstance)))
  (if (!= (Utilities|Array|Length (Variables|/Game/BluePrints/AbyssGameInstance.AbyssGameInstance_C|GetcheckpointId _asabyss_game_instance)) 0)
    (bind _outactors (Actor|GetAllActorsOfClass "/Game/BluePrints/Exploration/checkPoint.checkPoint_C"))
    (Default|StartFire (Utilities|Array|Get(acopy) _outactors (Utilities|Array|Get(acopy) (Variables|/Game/BluePrints/AbyssGameInstance.AbyssGameInstance_C|GetcheckpointId _asabyss_game_instance))))))

(event Custom|UpdateAnimation
  ;[1 1 1] Handle Animation
  (Sprite|SetFlipbook (Variables|Default|GetSprite) (select (> (Math|Vector|VectorLength (Transformation|GetVelocity)) 0.0) "/Game/Assets/Sprites/Character/Anim_Knight_Walk.Anim_Knight_Walk" "/Game/Assets/Sprites/Character/Anim_Knight_Idle.Anim_Knight_Idle")))

(event Custom|Flicker%20Light
  (bind _spotlight (Variables|Default|GetSpotLight))
  (bind _spotlight_2 (Variables|Default|GetSpotLight))
  (bind _returnvalue (Rendering|Components|Light|GetLightColor _spotlight))
  (bind _intensity (Variables|/Script/Engine.LightComponentBase|GetIntensity _spotlight_2))
  (bind (_r _g _b _a) (Utilities|Struct|BreakLinearColor _returnvalue))
  ;[1 1 1] Player Light Flicker
  (Utilities|FlowControl|Delay (Math|Random|RandomFloatinRange 0.1 0.6))
  (Utilities|FlowControl|FlipFlop
    (:A
      (Rendering|Components|Light|SetIntensity _spotlight_2 (* _intensity 1.15))
      (Rendering|Components|Light|SetLightColor _spotlight (Math|Color|MakeColor _r _g (- _b 0.05) _a) true))
    (:B
      (Rendering|Components|Light|SetIntensity _spotlight_2 (/ _intensity 1.15))
      (Rendering|Components|Light|SetLightColor _spotlight (Math|Color|MakeColor _r _g (+ _b 0.05) _a) true))))

(event Custom|relightTorches
  ;[1 1 1] Relight Lit Torches
  (bind _asabyss_game_instance (Utilities|Casting|CastToAbyssGameInstance (Game|GetGameInstance)))
  (for _array_element (Variables|/Game/BluePrints/AbyssGameInstance.AbyssGameInstance_C|GetlitTorches _asabyss_game_instance)
    (bind _outactors (Actor|GetAllActorsOfClass "/Game/BluePrints/Exploration/LightableTorch.LightableTorch_C"))
    (Variables|/Game/BluePrints/Exploration/LightableTorch.LightableTorch_C|SettorchIsLit (Utilities|Array|Get(acopy) _outactors _array_element) true)
    (Rendering|Components|Light|SetIntensity (Variables|/Game/BluePrints/Exploration/LightableTorch.LightableTorch_C|GetSpotLight (Utilities|Array|Get(acopy) _outactors _array_element)) (Variables|/Game/BluePrints/Exploration/LightableTorch.LightableTorch_C|GettorchIntensity (Utilities|Array|Get(acopy) _outactors _array_element)))
    (Rendering|SetVisibility (Variables|/Game/BluePrints/Exploration/LightableTorch.LightableTorch_C|GetSpotLight (Utilities|Array|Get(acopy) _outactors _array_element)) true false)))

(event Custom|playClimbing
  (bind _playerclimbing (Variables|Default|GetplayerClimbing))
  (bind _returnvalue (Audio|Components|Audio|IsPlaying _playerclimbing))
  ;[1 1 1] Player Climbing
  (if (and (!= (Variables|Default|GetclimbScaleValue) 0.0) (Variables|Default|GetisOnLadder))
    (if (not _returnvalue)
      (Audio|Components|Audio|Play _playerclimbing 0.0))
    (elif _returnvalue
      (Audio|Components|Audio|Stop _playerclimbing))))

(event Custom|play%20Footsteps
  (bind _playerfootsteps (Variables|Default|GetplayerFootsteps))
  (bind _returnvalue (Audio|Components|Audio|IsPlaying _playerfootsteps))
  ;[1 1 1] Player Footsteps
  (if (Math|Boolean|ANDBoolean (!= (Variables|Default|GetmoveScaleValue) 0.0) (not (Variables|Default|GetisOnLadder)) (not (Variables|Default|GetisJumping)) (not (AI|Components|NavMovement|IsFalling (Variables|Character|GetCharacterMovement))))
    (if (not _returnvalue)
      (Audio|Components|Audio|Play _playerfootsteps 0.0))
    (elif _returnvalue
      (Audio|Components|Audio|Stop _playerfootsteps))))

(event EventTick
  (params (DeltaSeconds :type Float%20%28single-precision%29))
  ;[1 1 1] Tick - Updates animation
  (Utilities|FlowControl|Sequence
    (:then_0
      (CallFunction|CheckReturnfromBattle))
    (:then_1
      (CallFunction|UpdateAnimation)
      (Math|Float|CompareFloat (.X (Math|Vector|BreakVector (Variables|/Script/Engine.MovementComponent|GetVelocity (Pawn|GetMovementComponent)))) 0.0
        (:>
          (Pawn|SetControlRotation (Pawn|GetController) (Math|Rotator|MakeRotator 0.0 0.0 0.0) :!label _label))
        (:==
          (if (Variables|Default|GetmovingRight)
            (goto _label)
            (else
              (Pawn|SetControlRotation (Pawn|GetController) (Math|Rotator|MakeRotator 0.0 0.0 1.8e+02) :!label _label_2))))
        (:<
          (goto _label_2))))
    (:then_2
      (CallFunction|PlayFootsteps)
      (CallFunction|PlayClimbing))
    (:then_3
      (CallFunction|FlickerLight))))

(event EventBeginPlay
  (bind _spotlight (Variables|Default|GetSpotLight))
  (bind _playerfootsteps (Variables|Default|GetplayerFootsteps))
  (bind _playerclimbing (Variables|Default|GetplayerClimbing))
  ;[1 1 1] Main
  (Utilities|FlowControl|Sequence
    (:then_0
      (Class|ActorComponent|SetIsReplicated (Variables|Default|GetSprite) true)
      (Variables|Default|SetplayerHealth 1e+02)
      (Variables|Default|SetplayerMaxHealth 1e+02)
      (Variables|Default|SetlevelExperience 0.0)
      (Variables|Default|SetexperienceToLvlUp 1e+02)
      (Variables|Default|SetplayerLevel 1)
      (Variables|Default|SetplayerMaxMpPoints 1e+01)
      (Variables|Default|SetplayerMpPoints 1e+01)
      (Variables|Default|SetmaxFootstepVolume 2.0)
      (Variables|Default|SetfootstepVolume 1.0))
    (:then_1
      (bind _returnvalue (UserInterface|CreateWidget "/Game/UMG/playerHUD.playerHUD_C" (Game|GetPlayerController 0)))
      (UserInterface|Viewport|AddtoViewport _returnvalue 0)
      (Variables|Default|SetgamePaused false)
      (bind _output_get (Variables|Default|SetplayerLightIntensity 1024.0))
      (Variables|Default|SetmaxLightIntensity 2048.0)
      (bind _output_get_2 (Variables|Default|SetplayerLightRadius 2e+02))
      (Rendering|Components|Light|SetIntensity _spotlight _output_get)
      (Rendering|Lighting|SetAttenuationRadius _spotlight _output_get_2)
      (if (Audio|Components|Audio|IsPlaying _playerfootsteps)
        (Audio|Components|Audio|Stop _playerfootsteps)
        (if (Audio|Components|Audio|IsPlaying _playerclimbing)
          (Audio|Components|Audio|Stop _playerclimbing))))))

(event EventOnLanded
  (params (Hit :type Hit%20Result%20Structure%20%28by%20ref%29))
  ;[1 1 1] Landing Sound
  (bind _returnvalue (Audio|CreateSound2D "/Game/Assets/Sounds/armoredPlayerFootsteps.armoredPlayerFootsteps" (Variables|Default|GetfootstepVolume)))
  (Audio|Components|Audio|Play _returnvalue 0.0)
  (Utilities|FlowControl|Delay 0.4)
  (Audio|Components|Audio|Stop _returnvalue))

(event Input|ActionEvents|InputActionJump
  (params (Key :type Key%20Structure :default "AnyKey"))
  ;[1 1 1] Handle Jump
  (:Pressed
    (Character|Jump)
    (Variables|Default|SetisJumping true))
  (:Released
    (Character|StopJumping)
    (Variables|Default|SetisJumping false)))

(event Input|AxisEvents|InputAxisClimb
  (params (AxisValue :type Float%20%28single-precision%29))
  ;[1 1 1] Climbing
  (Variables|Default|SetclimbScaleValue AxisValue))

(event Input|AxisEvents|InputAxisMoveRight
  (params (AxisValue :type Float%20%28single-precision%29))
  ;[1 1 1] Handle movement
  (if (> AxisValue 0.0)
    (Variables|Default|SetmovingRight true)
    (elif (< AxisValue 0.0)
      (Variables|Default|SetmovingRight false)))
  (Pawn|Input|AddMovementInput (Math|Vector|MakeVector (Variables|Default|GetmoveSpeed) 0.0 0.0) AxisValue false)
  (Variables|Default|SetmoveScaleValue AxisValue))

(event Input|KeyboardEvents|H
  (params (Key :type Key%20Structure :default "AnyKey"))
  ;[1 1 1] Test UI
  (:Pressed
    (Variables|Default|SetplayerHealth (- (Variables|Default|GetplayerHealth) 5.0))))

(event Input|KeyboardEvents|X
  (params (Key :type Key%20Structure :default "AnyKey"))
  ;[1 1 1] Test UI
  (:Pressed
    (Variables|Default|SetlevelExperience (+ (Variables|Default|GetlevelExperience) 5.0))))

(event Input|KeyboardEvents|P
  (params (Key :type Key%20Structure :default "AnyKey"))
  ;[1 1 1] Pause Menu
  (:Pressed
    (Utilities|IsValid (Variables|Default|GetpauseMenuReference)
      (:Is%20Valid
        _)
      (:Is%20Not%20Valid
        (bind _returnvalue (UserInterface|CreateWidget "/Game/UMG/pauseMenu.pauseMenu_C"))
        (Variables|Default|SetpauseMenuReference _returnvalue)))
    (Input|SetInputModeUIOnly (Game|GetPlayerController 0) (Variables|Default|GetpauseMenuReference) "LockAlways")
    (UserInterface|Viewport|AddtoViewport (Variables|Default|GetpauseMenuReference) 0)
    (Game|SetGamePaused true)))

(event Input|KeyboardEvents|L
  (params (Key :type Key%20Structure :default "AnyKey"))
  ;[1 1 1] Test UI
  (:Pressed
    (Variables|Default|SetplayerLevel (+ (Variables|Default|GetplayerLevel) 1))))

(event Input|KeyboardEvents|M
  (params (Key :type Key%20Structure :default "AnyKey"))
  ;[1 1 1] Test UI
  (:Pressed
    (Variables|Default|SetplayerMpPoints (- (Variables|Default|GetplayerMpPoints) 1.0))))

(event Input|TouchEvents|InputTouch
  (params (Location :type Vector) (FingerIndex :type ETouchIndex%20Enum))
  ;[1 1 1] Handle Jump
  (:Pressed
    (Character|Jump)
    (Variables|Default|SetisJumping true))
  (:Released
    (Character|StopJumping)
    (Variables|Default|SetisJumping false)))

(fn ConstructionScript)