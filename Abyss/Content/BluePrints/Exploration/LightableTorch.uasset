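; LightableTorch is an exploration torch that starts hidden and dark, then lights permanently when the cursor first passes over its Box.
; Hovering reveals the flipbook and restores SpotLight intensity, playing a 2D ignition sound only the first time.
; Tick fakes flicker through a random Delay and FlipFlop that alternately raise and lower intensity and shift the color's blue channel.
; MaxIntensity and MaxVolume are initialized but unused here.
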(event OnBeginCursorOver(Box)
  (params (TouchedComponent :type Primitive%20Component%20Object%20Reference))
  ;[1 1 1] Reveal on mouseover
  (Rendering|SetVisibility (Variables|Default|GetRenderComponent) true false)
  (Rendering|Components|Light|SetIntensity (Variables|Default|GetSpotLight) (Variables|Default|GettorchIntensity))
  (if (not (Variables|Default|GettorchIsLit))
    (Variables|Default|SettorchIsLit true)
    (Audio|PlaySound2D "/Game/Assets/Sounds/fireIgnite.fireIgnite" (Variables|Default|GetignitionVolume))))

(event EventTick
  (params (DeltaSeconds :type Float%20%28single-precision%29))
  (bind _spotlight (Variables|Default|GetSpotLight))
  (bind _spotlight_2 (Variables|Default|GetSpotLight))
  (bind _returnvalue (Rendering|Components|Light|GetLightColor _spotlight))
  (bind _intensity (Variables|/Script/Engine.LightComponentBase|GetIntensity _spotlight_2))
  (bind (_r _g _b _a) (Utilities|Struct|BreakLinearColor _returnvalue))
  ;[1 1 1] Light Flicker
  (Utilities|FlowControl|Delay (Math|Random|RandomFloatinRange 0.1 0.6))
  (Utilities|FlowControl|FlipFlop
    (:A
      (Rendering|Components|Light|SetIntensity _spotlight_2 (* _intensity 1.15))
      (Rendering|Components|Light|SetLightColor _spotlight (Math|Color|MakeColor _r _g (- _b 0.05) _a) true))
    (:B
      (Rendering|Components|Light|SetIntensity _spotlight_2 (/ _intensity 1.15))
      (Rendering|Components|Light|SetLightColor _spotlight (Math|Color|MakeColor _r _g (+ _b 0.05) _a) true))))

(event EventBeginPlay
  ;[1 1 1] Hide light and flipbook
  (Rendering|SetVisibility (Variables|Default|GetRenderComponent) false false)
  (Rendering|Components|Light|SetIntensity (Variables|Default|GetSpotLight) 0.0)
  (Variables|Default|SettorchIntensity 512.0)
  (Variables|Default|SetmaxIntensity 1024.0)
  (Variables|Default|SettorchIsLit false)
  (Variables|Default|SetignitionVolume 1.0)
  (Variables|Default|SetmaxVolume 2.0))

(fn ConstructionScript)