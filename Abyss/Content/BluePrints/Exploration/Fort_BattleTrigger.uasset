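; Exploration trigger actor that starts a fort battle when any actor overlaps it.
; On overlap it picks a uniformly random entry from its EnemyTable and stores it in AbyssGameInstance's EnemyToFightStruct, so the choice survives the level change.
; It then opens the Fort_Battle level, with no filter on which actor overlapped.
; A random-stream node is left unconnected and never runs.
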(event EventBeginPlay)

(event Collision|EventActorBeginOverlap
  (params (OtherActor :type Actor%20Object%20Reference))
  (bind _enemytable (Variables|Default|GetEnemyTable))
  ;[1 1 1] Choose Enemy to Fight from Loot Table
  (bind _asabyss_game_instance (Utilities|Casting|CastToAbyssGameInstance (Game|GetGameInstance)))
  (Variables|/Game/BluePrints/AbyssGameInstance.AbyssGameInstance_C|SetEnemyToFightStruct _asabyss_game_instance (Utilities|Array|Get(acopy) _enemytable (Math|Random|RandomIntegerinRange 0 (- (Utilities|Array|Length _enemytable) 1))))
  ;[1 1 1] Travel to Battle Level
  (Game|OpenLevel(byName) "Fort_Battle"))

(event EventTick
  (params (DeltaSeconds :type Float%20%28single-precision%29)))

(fn ConstructionScript)