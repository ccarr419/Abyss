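; Ladder actor for exploration that notifies the player's Exploration_Hero when it is on a ladder.
; Every Tick, it takes the first Exploration_Hero in the level and tests its overlap against all Ladder actors, not just itself.
; On a match it calls OnLadder on the hero, while the False branch has no follow-up in the event graph.
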(event EventTick
  (params (DeltaSeconds :type Float%20%28single-precision%29))
  ;[1 1 1] Find if the Player is on the Ladder
  (bind _overlappingplayer (Utilities|FindifPlayerIsonLadder)
    (:True
      (Default|OnLadder _overlappingplayer))))

(fn ConstructionScript)