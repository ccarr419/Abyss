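; Ladder actor that puts the exploration hero into ladder behavior while the hero overlaps a ladder.
; Each Tick it finds the first Exploration_Hero and runs checkIfOverlapping, calling OnLadder on the hero when the result is true.
; The check loops over every Ladder in the level and stops at the first overlap, so each instance polls all ladders rather than using overlap events.
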(event EventBeginPlay)

(event Collision|EventActorBeginOverlap
  (params (OtherActor :type Actor%20Object%20Reference)))

(event EventTick
  (params (DeltaSeconds :type Float%20%28single-precision%29))
  (bind _outactors (Actor|GetAllActorsOfClass "/Game/BluePrints/Exploration/Exploration_Hero.Exploration_Hero_C"))
  (if (Utilities|IsValid (Utilities|Array|Get(acopy) _outactors))
    (bind _isonladder (Utilities|CheckifOverlapping (Utilities|Array|Get(acopy) _outactors))
      (:Exit
        (if _isonladder
          (Default|OnLadder (Utilities|Array|Get(acopy) _outactors)))))))

(fn ConstructionScript)